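; Base item actor that shows a text prompt when a character is nearby and can be picked up into a backpack.
; Overlap events store the character and toggle the text and interaction flags, while Tick turns the text toward BP_ThirdPersonCharacter's follow camera.
; Interact passes the character's BP_BackpackComponent to PutIntoBackpack, an empty stub here, and returns true on every path.
; AfterUse destroys the actor.
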(event EventBeginPlay
  (Rendering|SetVisibility (Variables|Default|GetTextRender) false false))

(event Collision|EventActorBeginOverlap
  (params (OtherActor :type Actor%20Object%20Reference))
  (bind _ascharacter (Utilities|Casting|CastToCharacter OtherActor))
  (Variables|Default|SetCharacterInBox _ascharacter)
  (Rendering|SetVisibility (Variables|Default|GetTextRender) true false)
  (Variables|Default|SetIsReadyTolnteract true)
  (Variables|Default|SetIsLookAtPlayerCamera true))

(event Collision|EventActorEndOverlap
  (params (OtherActor :type Actor%20Object%20Reference))
  (Utilities|Casting|CastToCharacter OtherActor)
  (Variables|Default|SetCharacterInBox 0)
  (Rendering|SetVisibility (Variables|Default|GetTextRender) false false)
  (Variables|Default|SetIsReadyTolnteract false)
  (Variables|Default|SetIsLookAtPlayerCamera false))

(event EventTick
  (params (DeltaSeconds :type Float%20%28single-precision%29))
  (CallFunction|LookingatPlayerCamera))

(fn ConstructionScript)

(fn LookingatPlayerCamera
  (if (Variables|Default|GetIsLookAtPlayerCamera)
    (bind _characterinbox (Variables|Default|GetCharacterInBox)
      (:then
        (bind _asbp_third_person_character (Utilities|Casting|CastToBP_ThirdPersonCharacter _characterinbox))
        (Variables|Default|SetL_CameraLocation (Transformation|GetWorldLocation (Variables|/Game/Blueprints/Characters/BP_ThirdPersonCharacter.BP_ThirdPersonCharacter_C|GetFollowCamera _asbp_third_person_character)))
        (Transformation|SetWorldRotation (Variables|Default|GetTextRender) (Math|Rotator|FindLookatRotation (Transformation|GetWorldLocation (Variables|Default|GetTextRender)) (Variables|Default|GetL_CameraLocation)) false false))
      (:else))))

(fn PutIntoBackpack
  (params (InBackpack :type BP%20Backpack%20Component%20Object%20Reference)))

(fn AfterUse
  (Actor|DestroyActor))

(fn Interact
  (if (Variables|Default|GetIsReadyTolnteract)
    (bind _characterinbox (Variables|Default|GetCharacterInBox)
      (:then
        (Utilities|IsValid (Actor|GetComponentbyClass _characterinbox "/Game/Blueprints/Components/BP_BackpackComponent.BP_BackpackComponent_C")
          (:Is%20Valid
            (CallFunction|PutIntoBackpack (Actor|GetComponentbyClass _characterinbox "/Game/Blueprints/Components/BP_BackpackComponent.BP_BackpackComponent_C"))
            (return true))
          (:Is%20Not%20Valid
            (return true))))
      (:else
        (return true)))
    (else
      (return true))))