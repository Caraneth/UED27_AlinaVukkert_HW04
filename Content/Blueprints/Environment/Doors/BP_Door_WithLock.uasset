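; Lockable child door that opens only while unlocked and shows lock state with a red or green indicator light.
; Interact toggles an unlocked door; on a locked one it checks the overlapping actor's BP_BackpackComponent for required quest items and unlocks if all are found.
; Matched keys are removed during the check, even when the set is incomplete.
; SwitchLock and Unlock change state directly, while Lock works only on doors without required keys.
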(event EventBeginPlay
  (|CallParentFunction) ; This node is disabled and will not be called.\nDrag off pins to build functionality.
)

(event Collision|EventActorBeginOverlap
  (params (OtherActor :type Actor%20Object%20Reference))
  (|CallParentFunction OtherActor) ; This node is disabled and will not be called.\nDrag off pins to build functionality.
)

(event EventTick
  (params (DeltaSeconds :type Float%20%28single-precision%29))
  (|CallParentFunction DeltaSeconds) ; This node is disabled and will not be called.\nDrag off pins to build functionality.
)

(event EventOpenDoor
  (if (not (Variables|DoorConfigure|GetIsDoorLoked))
    (|CallParentFunction)))

(event EventCloseDoor
  (|CallParentFunction))

(fn ConstructionScript
  (|CallParentFunction)
  (CallFunction|UpdateDoorLockIndication))

(fn SwitchLock
  (Variables|DoorConfigure|SetIsDoorLoked (not (Variables|DoorConfigure|GetIsDoorLoked)))
  (CallFunction|UpdateDoorLockIndication))

(fn UpdateDoorLockIndication
  (Rendering|Components|Light|SetLightColor (Variables|Default|GetPointLockindicatorLight) (Math|Color|SelectColor "(R=0.557292,G=0.000000,B=0.026066,A=1.000000)" "(R=0.062801,G=1.000000,B=0.000000,A=1.000000)" (Variables|DoorConfigure|GetIsDoorLoked)) true))

(fn Lock
  (if (not (Utilities|Array|IsValidIndex (Variables|Default|GetNeededKeysName)))
    (Variables|DoorConfigure|SetIsDoorLoked true)
    (CallFunction|UpdateDoorLockIndication)))

(fn Unlock
  (Variables|DoorConfigure|SetIsDoorLoked false)
  (CallFunction|UpdateDoorLockIndication))

(fn Interact
  (if (Variables|Default|GetIs%20Ready%20to%20Interact)
    (if (not (Variables|DoorConfigure|GetIsDoorLoked))
      (if (Variables|Default|GetIsDoorOpen)
        (CallFunction|CloseDoor)
        (return true)
        (else
          (CallFunction|OpenDoor)
          (return true)))
      (elif (Utilities|Array|IsValidIndex (Variables|Default|GetNeededKeysName))
        (bind _overlappedactor (Variables|Default|GetOverlappedActor)
          (:then
            (Utilities|IsValid (Actor|GetComponentbyClass _overlappedactor "/Game/Blueprints/Components/BP_BackpackComponent.BP_BackpackComponent_C")
              (:Is%20Valid
                (LocalVariables|SetL_Backpack (Actor|GetComponentbyClass _overlappedactor "/Game/Blueprints/Components/BP_BackpackComponent.BP_BackpackComponent_C"))
                (for _array_element (Variables|Default|GetNeededKeysName)
                  (LocalVariables|SetL_ItemName _array_element)
                  (if (Utilities|Set|Contains (Variables|/Game/Blueprints/Components/BP_BackpackComponent.BP_BackpackComponent_C|GetQuestItems (LocalVariables|GetL_Backpack)) (LocalVariables|GetL_ItemName))
                    (Math|Integer|IncrementInt (LocalVariables|GetL_ItemInrement)
                      (:%20%20
                        ;[0.06616 0.245 0.2552] Remove item from inventory after use
                        (Default|RemoveQuestItem (LocalVariables|GetL_Backpack) (LocalVariables|GetL_ItemName))))))
                (if (== (LocalVariables|GetL_ItemInrement) (Utilities|Array|Length (Variables|Default|GetNeededKeysName)))
                  (CallFunction|Unlock)
                  (else
                    (return true))))
              (:Is%20Not%20Valid
                (return true))))
          (:else
            (return true)))
        (else
          (return true))))
    (else
      (return false))))