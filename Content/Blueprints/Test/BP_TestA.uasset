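; BP_TestA is a test Blueprint that exercises custom events, functions and local variables.
; BeginPlay calls a print event directly and through NewFunction0, which multiplies an integer by five via MultByFive, forwards it as a float and returns it.
; The event prints its bool and float parameters on screen, with the text color chosen by the bool.
; The second custom event, Tick, construction script and NewFunction1 are empty stubs.
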(event Custom|CustomEvent_0
  (params (InNewParam :type Boolean) (InNewParam2 :type Byte) (InNewParam3 :type Float%20%28single-precision%29) (InNewParam4 :type String))
  (Development|PrintString (Utilities|String|Append "Bool =" (Utilities|String|ToString(Boolean) InNewParam) "Float =" (Utilities|String|ToString(Float) InNewParam3) " !") true false (Math|Color|SelectColor "(R=0.080202,G=0.583333,B=0.140131,A=1.000000)" "(R=0.619792,G=0.054407,B=0.116194,A=1.000000)" InNewParam) 5.0))

(event Custom|CustomEvent_1)

(event EventBeginPlay
  (CallFunction|CustomEvent0 false 0 0.0)
  (CallFunction|CustomEvent0 true 0 0.0)
  (CallFunction|NewFunction0 "" (Class|KismetSystemLibrary|MakeLiteralBool false) 1))

(event Collision|EventActorBeginOverlap
  (params (OtherActor :type Actor%20Object%20Reference)))

(event EventTick
  (params (DeltaSeconds :type Float%20%28single-precision%29)))

(fn ConstructionScript)

(fn NewFunction0
  (params (InName :type String) (InArray :type Boolean) (InInt :type Integer))
  (Utilities|FlowControl|Sequence
    (:then_3
      (if true
        (bind _newparam1 (CallFunction|MultbyFive InInt))
        (LocalVariables|SetL_Int _newparam1)
        (CallFunction|CustomEvent0 InArray 0 (Math|Conversions|ToFloat(Integer) (LocalVariables|GetL_Int)) InName)
        (CallFunction|CustomEvent1)
        (return (LocalVariables|GetL_Int))
        (else
          (return 0))))))

(fn NewFunction1)

(fn MultbyFive
  (params (NewParam :type Integer))
  (return (* NewParam 5)))